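; BP_Timer is a simple timer actor that tracks elapsed time in minute and second counters.
; On BeginPlay it waits one second, increments the seconds counter, then rolls it over into minutes once it passes 59.
; The chain has no loop back to the delay and Tick is empty, so the count advances only once per BeginPlay.
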(event EventBeginPlay
  (Utilities|FlowControl|Delay 1.0)
  (Variables|Default|SetSecondss (+ (Variables|Default|GetSecondss) 1))
  (if (> (Variables|Default|GetSecondss) 59)
    (Variables|Default|SetMinutess (+ (Variables|Default|GetMinutess) 1))
    (Variables|Default|SetSecondss 0)))

(event Collision|EventActorBeginOverlap
  (params (OtherActor :type Actor%20Object%20Reference)))

(event EventTick
  (params (DeltaSeconds :type Float%20%28single-precision%29)))

(fn ConstructionScript)
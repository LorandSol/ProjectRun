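; Grappling hook component for BP_ThirdPersonMain that pulls the character to BP_GrappleTarget actors, driven by a four-state machine on Tick.
; While retracted, it highlights the visible target in range closest to the camera's forward direction.
; AttemptGrapple spawns a hook and a hand-attached cable line.
; As the hook nears its target, the character hops, flies toward it from the apex, then launches onward and clears the grapple.
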(event EventBeginPlay
  (bind _asbp_third_person_main (Utilities|Casting|CastToBP_ThirdPersonMain (Components|GetOwner)))
  (Variables|Private|SetOwningCharacter _asbp_third_person_main))

(event EventTick
  (params (DeltaSeconds :type Float%20%28single-precision%29))
  (switch Utilities|FlowControl|Switch|SwitchonE_GrappleState (Variables|Private|GetGrappleState)
    (:NewEnumerator0
      (CallFunction|TickRetracted))
    (:NewEnumerator1
      (CallFunction|TickFiring))
    (:NewEnumerator2
      (CallFunction|TickNearingTarget))
    (:NewEnumerator3
      (CallFunction|TickonTarget))))

(fn TickRetracted
  (bind _outactors (Collision|SphereOverlapActors (Transformation|GetActorLocation (Variables|Private|GetOwningCharacter)) (Variables|Private|GetMaxGrappleDistance) (Utilities|Array|MakeArray "ObjectTypeQuery1") "/Game/JaredStuff/Grappling/Blueprints/BP_GrappleTarget.BP_GrappleTarget_C"))
  (bind _target (CallFunction|FindBestTarget _outactors))
  (CallFunction|SetCurrentTarget (.AsBP%20Grapple%20Target (Utilities|Casting|CastToBP_GrappleTarget _target))))

(fn TickFiring
  (if (< (Default|DistancetoTarget (Variables|Default|GetGrappleHook)) (Variables|Default|GetStartJumpDistance))
    (Character|LaunchCharacter (Variables|Private|GetOwningCharacter) "0.000000,0.000000,500.000000" true true)
    (Variables|Private|SetGrappleState "NewEnumerator2")))

(fn TickNearingTarget
  (if (<= (.z (Transformation|GetVelocity (Variables|Private|GetOwningCharacter))) 0.0)
    (Variables|Default|SetInitialDirection (Utilities|OwnertoTarget))
    (Variables|Private|SetGrappleState "NewEnumerator3")))

(fn TickonTarget
  (bind _initialdirection (Variables|Default|GetInitialDirection))
  (bind _returnvalue (* _initialdirection 1e+02))
  (if (< (Transformation|GetDistanceTo (Variables|Private|GetOwningCharacter) (Variables|Private|GetCurrentTarget)) (Variables|Default|GetEndJumpDistance))
    (Character|LaunchCharacter (Variables|Private|GetOwningCharacter) (Math|Vector|MakeVector (.x _returnvalue) (.y _returnvalue) (Math|Float|Max(Float) (.z _returnvalue) 5e+02)) true true)
    (CallFunction|SetCurrentTarget)
    (Actor|DestroyActor (Variables|Default|GetGrappleLine))
    (Variables|Default|SetGrappleLine 0)
    (Actor|DestroyActor (Variables|Default|GetGrappleHook))
    (Variables|Default|SetGrappleHook 0)
    (Variables|Private|SetGrappleState "NewEnumerator0")
    (else
      (Variables|/Script/Engine.MovementComponent|SetVelocity (Pawn|GetMovementComponent (Variables|Private|GetOwningCharacter)) (* (Utilities|OwnertoTarget) (Variables|Default|GetCharacterGrappleSpeed))))))

(fn FindBestTarget
  (params (Targets :type Array%20of%20Actor%20Object%20References))
  (bind _owningcharacter (Variables|Private|GetOwningCharacter))
  (for _array_element Targets
    (LocalVariables|SetCurrentTarget%20%28Local%29 _array_element)
    (bind (_outhit _returnvalue) (Collision|LineTraceByChannel (Transformation|GetActorLocation (Variables|Private|GetOwningCharacter)) (Transformation|GetActorLocation (LocalVariables|GetCurrentTarget%20%28Local%29)) "TraceTypeQuery1" false (Utilities|Array|MakeArray (Variables|Private|GetOwningCharacter)) "None" true "(R=1.000000,G=0.000000,B=0.000000,A=1.000000)" "(R=0.000000,G=1.000000,B=0.000000,A=1.000000)" 0.5))
    (if _returnvalue
      (if (== (.HitActor (Collision|BreakHitResult _outhit)) (LocalVariables|GetCurrentTarget%20%28Local%29))
        (Utilities|FlowControl|Sequence
          (:then_0
            ;[1 1 1] Step 1) Calculate Angle to Target
            (LocalVariables|SetCurrentAngle%20%28Local%29 (Class|KismetMathLibrary|DegAcos (Math|Vector|DotProduct (Math|Vector|Normalize (- (Transformation|GetActorLocation (LocalVariables|GetCurrentTarget%20%28Local%29)) (Transformation|GetActorLocation _owningcharacter))) (Math|Vector|GetForwardVector (Variables|/Game/LaylaStuff/BP_ThirdPersonMain.BP_ThirdPersonMain_C|GetFollowCamera _owningcharacter))))))
          (:then_1
            ;[1 1 1] Step 2) If angle < current angle, make this the new target
            (if (or (< (LocalVariables|GetCurrentAngle%20%28Local%29) (LocalVariables|GetBestAngle%20%28Local%29)) (not (Utilities|IsValid (LocalVariables|GetBestTarget%20%28Local%29))))
              (LocalVariables|SetBestTarget%20%28Local%29 (LocalVariables|GetCurrentTarget%20%28Local%29))
              (LocalVariables|SetBestAngle%20%28Local%29 (LocalVariables|GetCurrentAngle%20%28Local%29))))))))
  (return (LocalVariables|GetBestTarget%20%28Local%29)))

(fn SetCurrentTarget
  (params (NewTarget :type BP%20Grapple%20Target%20Object%20Reference))
  (if (!= NewTarget (Variables|Private|GetCurrentTarget))
    (Utilities|FlowControl|Sequence
      (:then_0
        (bind _currenttarget (Variables|Private|GetCurrentTarget)
          (:then
            (Default|SetActive _currenttarget false))
          (:else)))
      (:then_1
        (Variables|Private|SetCurrentTarget NewTarget))
      (:then_2
        (bind _currenttarget_2 (Variables|Private|GetCurrentTarget)
          (:then
            (Default|SetActive _currenttarget_2 true))
          (:else))))))

(fn AttemptGrapple
  (switch Utilities|FlowControl|Switch|SwitchonE_GrappleState (Variables|Private|GetGrappleState)
    (:NewEnumerator0
      (bind _currenttarget (Variables|Private|GetCurrentTarget)
        (:then
          (bind _returnvalue (Game|SpawnActorfromClass "/Game/JaredStuff/Grappling/Blueprints/BP_GrappleHook.BP_GrappleHook_C" (Math|Transform|MakeTransform (Utilities|OwnerLocation) "0, 0, 0" "1.000000,1.000000,1.000000") "AlwaysSpawn" "MultiplyWithRoot" 0 _currenttarget 5e+03 0))
          (Variables|Default|SetGrappleHook _returnvalue)
          (bind _returnvalue_2 (Game|SpawnActorfromClass "/Game/JaredStuff/Grappling/Blueprints/BP_GrappleLine.BP_GrappleLine_C" (Math|Transform|MakeTransform (Utilities|OwnerLocation) "0, 0, 0" "1.000000,1.000000,1.000000") "AlwaysSpawn" "MultiplyWithRoot" 0 0))
          (bind _output_get (Variables|Default|SetGrappleLine _returnvalue_2))
          (Transformation|AttachComponentToComponent _output_get (Variables|/Script/Engine.Character|GetMesh (Variables|Private|GetOwningCharacter)) "hand_r" "SnapToTarget" "SnapToTarget" "SnapToTarget" true)
          (Class|CableComponent|SetAttachEndto (Variables|/Script/CableComponent.CableActor|GetCableComponent (Variables|Default|GetGrappleLine)) (Variables|Default|GetGrappleHook) "DefaultSceneRoot" "None")
          (Transformation|SetActorRotation (Variables|Private|GetOwningCharacter) (Math|Rotator|MakeRotfromZX (Math|Vector|MakeVector 0.0 0.0 1.0) (Utilities|OwnertoTarget)))
          (Variables|Private|SetGrappleState "NewEnumerator1"))
        (:else)))))
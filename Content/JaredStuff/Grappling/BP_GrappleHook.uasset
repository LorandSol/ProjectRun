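; BP_GrappleHook is a grapple hook projectile that launches toward a target actor when it spawns.
; On BeginPlay it stores its own and the Target's locations, normalizes the vector between them and scales it by Speed to set the ProjectileMovement velocity.
; The direction is computed only once, and the event graph holds no attach, pull or hit logic.
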(event EventBeginPlay
  (Variables|Default|SetStartLocation (Transformation|GetActorLocation))
  (Variables|Default|SetEndLocation (Transformation|GetActorLocation (Variables|Default|GetTarget)))
  (Variables|Default|SetDirection (Math|Vector|Normalize (- (Variables|Default|GetEndLocation) (Variables|Default|GetStartLocation))))
  (Variables|/Script/Engine.MovementComponent|SetVelocity (Variables|Default|GetProjectileMovement) (* (Variables|Default|GetDirection) (Variables|Default|GetSpeed))))

(fn ConstructionScript)